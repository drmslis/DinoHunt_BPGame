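; Player pawn for a dinosaur board game, holding identity, color, diamonds, traps, cards, collected dinos and turns to skip.
; SlideStep recursively consumes a tile track using position and rotation timelines, while PawnJumpMove arcs directly to a target tile.
; Finished moves call the game mode to arrange pawns, then trigger either the salary shop or the landed tile's event.
; Helper functions manage resources, total dino points and random trap or dino losses.
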(event Custom|LoseDino
  (bind _playerdinos (Variables|Default|GetPlayerDinos))
  (bind _returnvalue (Utilities|Array|LastIndex _playerdinos))
  (bind _returnvalue_2 (Math|Random|RandomIntegerinRange 0 _returnvalue))
  (bind _output (Utilities|Array|Get(acopy) _playerdinos _returnvalue_2))
  ;[1 1 1] LoseDino
  (if (not (== (Utilities|Array|Length _playerdinos) 0))
    (Development|PrintString (Utilities|String|Append "У вас сбежал: " (Utilities|String|ToString(Name) (.dinoname _output)) " Вы теряете: " (Utilities|String|ToString(Integer) (.dinocost _output)) " очков") true true "(R=1.000000,G=0.000000,B=0.041135,A=1.000000)" 5.0)
    (Utilities|Array|RemoveIndex _playerdinos _returnvalue_2)
    (CallFunction|SummDinoPoints)))

(event Custom|TestClearCardArray
  (Utilities|Array|Clear (Variables|Default|GetCardsOnHands)))

(event Custom|ToggleLight
  (if (Rendering|IsVisible (Variables|Default|GetPointLight))
    (Rendering|SetVisibility (Variables|Default|GetPointLight) false false)
    (else
      (Rendering|SetVisibility (Variables|Default|GetPointLight) true false))))

(event Custom|SlideStep
  (params (IsLoopPassed :type Boolean))
  (Variables|Default|SetIsLoopPassed IsLoopPassed)
  (Variables|Movement|SetCurrentLocIndex (Utilities|Array|Get(acopy) (Variables|Movement|GetMoveTrack)))
  (Utilities|Array|RemoveIndex (Variables|Movement|GetMoveTrack))
  (Variables|Movement|SetTargetLoc (.TilePos (Default|GetTilePosRot (Variables|Default|GetBP_GameModeRef) (Variables|Movement|GetCurrentLocIndex))))
  (Variables|Movement|SetTargetRot (.TileRot (Default|GetTilePosRot (Variables|Default|GetBP_GameModeRef) (Variables|Movement|GetCurrentLocIndex))))
  (Variables|Movement|SetCurrentLoc (Transformation|GetActorLocation self))
  (Variables|Movement|SetCurrentRot (Transformation|GetActorRotation self))
  (if (> (Utilities|Array|Length (Variables|Movement|GetMoveTrack)) 0)
    (bind _duration (Timeline|TileLineSlideSlow PlayFromStart)
      (:Update
        (Transformation|SetActorRelativeLocation self (Math|Vector|Lerp(Vector) (Variables|Movement|GetCurrentLoc) (Variables|Movement|GetTargetLoc) _duration)))
      (:Finished
        (Default|PlayersPoser (Variables|Default|GetBP_GameModeRef))
        (bind _rotator (Timeline|TimeineSlideRotator PlayFromStart)
          (:Update
            (Transformation|SetActorRotation (Math|Rotator|Lerp(Rotator) (Variables|Movement|GetCurrentRot) (Variables|Movement|GetTargetRot) _rotator true)))
          (:Finished
            (CallFunction|SlideStep (Variables|Default|GetIsLoopPassed))))))
    (else
      (bind _duration_2 (Timeline|TimeLineSlideFast PlayFromStart)
        (:Update
          (Transformation|SetActorRelativeLocation self (Math|Vector|Lerp(Vector) (Variables|Movement|GetCurrentLoc) (Variables|Movement|GetTargetLoc) _duration_2)))
        (:Finished
          (Default|PlayersPoser (Variables|Default|GetBP_GameModeRef))
          (if (Variables|Default|GetIsLoopPassed)
            (Default|Shop (Variables|Default|GetBP_GameModeRef) self true)
            (else
              (Default|ActivateTile (Variables|Default|GetBP_GameModeRef) (Variables|Movement|GetCurrentLocIndex)))))))))

(event Custom|Init
  (params (BP_GameModeRef :type BP%20Game%20Mod%20Object%20Reference) (PlayerName :type String) (PlayerColor :type Vector) (PlayerNumber :type Integer))
  (Variables|Default|SetBP_GameModeRef BP_GameModeRef)
  (Variables|Default|SetPlayerName PlayerName)
  (Variables|Default|SetPlayerColor PlayerColor)
  (Variables|Default|SetPlayerNumber PlayerNumber)
  (Rendering|Material|SetVectorParameterValueonMaterials (Variables|Default|GetSkeletalMesh) "PlayerColor" (Variables|Default|GetPlayerColor))
  (Rendering|Components|Light|SetLightColor (Variables|Default|GetPointLight) (Utilities|Struct|MakeLinearColor (.x (Variables|Default|GetPlayerColor)) (.y (Variables|Default|GetPlayerColor)) (.z (Variables|Default|GetPlayerColor)) 1.0) true))

(event Custom|LoseTrap
  (bind _activetraps (Variables|Default|GetActiveTraps))
  (bind _returnvalue (Utilities|Array|LastIndex _activetraps))
  (bind _returnvalue_2 (Math|Random|RandomIntegerinRange 0 _returnvalue))
  ;[1 1 1] LoseTrap
  (if (not (== (Utilities|Array|Length _activetraps) 0))
    (Default|DestroyTrap (Utilities|Array|Get(acopy) _activetraps _returnvalue_2))
    (Utilities|Array|RemoveIndex _activetraps _returnvalue_2)))

(event Custom|AddTraps
  (params (HowMuch :type Integer))
  ;[1 1 1] Change Player Resources
  (Variables|Default|SetTraps (+ HowMuch (Variables|Default|GetTraps))))

(event Custom|LoseTurnSetter
  (params (HowMuchTurns :type Integer))
  (Variables|Default|SetTurnsToSkip (+ HowMuchTurns (Variables|Default|GetTurnsToSkip))))

(event Custom|PawnJumpMove
  (params (TileRef :type BP%20Tile%20Def%20Object%20Reference) (IsForwardJump :type Boolean))
  (bind _returnvalue (Transformation|GetActorLocation TileRef))
  (bind _returnvalue_2 (Transformation|GetActorRotation TileRef))
  (bind _self self)
  (bind _self_2 self)
  (bind _returnvalue_3 (Transformation|GetActorLocation _self))
  (Variables|Default|SetIsJumpForward IsForwardJump)
  (Default|SetTurnButtonState (Variables|/Game/BP/BP_GameMod.BP_GameMod_C|GetInGameUI (Variables|Default|GetBP_GameModeRef)) "Collapsed")
  (bind _jump (Timeline|TimeLineJumpMove PlayFromStart)
    (:Update
      (Transformation|SetActorLocation (Math|Vector|MakeVector (Math|Float|Lerp (.x _returnvalue_3) (.x _returnvalue) (.x _jump)) (Math|Float|Lerp (.y _returnvalue_3) (.y _returnvalue) (.y _jump)) (Math|Float|Lerp 0.0 1.5e+02 (.z _jump))) false false))
    (:Finished
      (if (Math|Rotator|Equal(Rotator) (Transformation|GetActorRotation self) _returnvalue_2 0.0001)
        (Development|PrintString "Уииииии!" true true "(R=1.000000,G=0.000000,B=0.018539,A=1.000000)" :!label _label)
        (Variables|Movement|SetCurrentLocIndex (Variables|/Game/BP/Tiles/Bp_TileDef.BP_TileDef_C|GetNumber TileRef))
        (Default|PlayersPoser (Variables|Default|GetBP_GameModeRef))
        (if (and (Variables|Default|GetIsJumpForward) (== (CallFunction|GetPlayerCurrentPos) 0))
          (Default|Shop (Variables|Default|GetBP_GameModeRef) self true)
          (else
            (Class|TileEvent|EnterEvent(Message) TileRef self)))
        (else
          (bind _rotator (Timeline|TimeLineJumpRotator PlayFromStart)
            (:Update
              (Transformation|SetActorRotation _self_2 (Math|Rotator|Lerp(Rotator) (Transformation|GetActorRotation _self_2) _returnvalue_2 _rotator true)))
            (:Finished
              (goto _label))))))))

(event Custom|GetSlideTrack
  (params (Track :type Array%20of%20Integers) (IsLoop :type Boolean))
  (Variables|Movement|SetMoveTrack Track)
  (CallFunction|SlideStep IsLoop))

(fn ConstructionScript)

(fn IsCardonHand
  (params (ItemToFind :type E_SafeItems%20Enum%20%28by%20ref%29 :default "NewEnumerator0"))
  (return (Utilities|Array|FindItem (Variables|Default|GetCardsOnHands) ItemToFind)))

(fn SpendDiamonds
  (params (HowMuch :type Integer) (CanPay :type Boolean) (ForceToZero :type Boolean))
  (if CanPay
    (Variables|Default|SetDiamonds (- (Variables|Default|GetDiamonds) (Math|Integer|Absolute(Integer) HowMuch)))
    (return HowMuch)
    (elif ForceToZero
      (LocalVariables|SetNewSumm (Variables|Default|GetDiamonds))
      (Variables|Default|SetDiamonds 0)
      (return (LocalVariables|GetNewSumm))
      (else
        (return 0)))))

(fn CheckDiamonds
  (params (Cost :type Integer))
  (return (>= (Variables|Default|GetDiamonds) Cost) Cost))

(fn SummDinoPoints
  (for _array_element (Variables|Default|GetPlayerDinos)
    (LocalVariables|SetSumm (+ (LocalVariables|GetSumm) (.dinocost _array_element))))
  (Variables|Default|SetDinoPoints (LocalVariables|GetSumm)))

(fn GetPlayerCurrentPos
  (return (Variables|Movement|GetCurrentLocIndex)))

(fn GetPlayerColor
  (return (Variables|Default|GetPlayerColor)))

(fn SetPlayerColor
  (params (PlayerColor :type Vector))
  (Variables|Default|SetPlayerColor PlayerColor))

(fn GetDinoPoints
  (return (Variables|Default|GetDinoPoints)))

(fn GetDiamonds
  (return (Variables|Default|GetDiamonds)))

(fn GetTrapsAmount
  (return (Variables|Default|GetTraps)))

(fn GetPlayerName
  (return (Variables|Default|GetPlayerName)))

(fn AddDiamonds
  (params (Value :type Integer))
  (Variables|Default|SetDiamonds (+ Value (Variables|Default|GetDiamonds))))

(fn SetTurnstoSkip
  (params (TurnsToSkip :type Integer))
  (Variables|Default|SetTurnsToSkip (Math|Integer|Clamp(Integer) TurnsToSkip 0 2)))

(fn GetTurnstoSkip
  (return (Variables|Default|GetTurnsToSkip)))

(fn OneTurnSkipped
  (bind _result (Math|Integer|DecrementInt (Variables|Default|GetTurnsToSkip))
    (:%20%20
      (bind _output_get (Variables|Default|SetTurnsToSkip (Math|Integer|Clamp(Integer) _result 0 999)))
      (return _output_get))))

(fn AddDino
  (params (Dino%20Name :type Name) (Dino%20Cost :type Integer))
  (Utilities|Array|Add (Variables|Default|GetPlayerDinos) (Utilities|Struct|MakePlayersDinos Dino%20Name Dino%20Cost))
  (CallFunction|SummDinoPoints))

(fn SpendTrap
  (if (> (Variables|Default|GetTraps) 0)
    (bind _result (Math|Integer|DecrementInt (Variables|Default|GetTraps))
      (:%20%20
        (return _result)))
    (else
      (return -1))))

(fn GetPlayerNumber
  (return (Variables|Default|GetPlayerNumber)))

(fn AddOwnedTrap
  (params (BP_Hunt :type BP%20Hunt%20Tile%20Object%20Reference))
  (Utilities|Array|Add (Variables|Default|GetActiveTraps) BP_Hunt))

(fn AddCardtoHand
  (params (NewItem :type E_SafeItems%20Enum%20%28by%20ref%29 :default "NewEnumerator0"))
  (Utilities|Array|Add (Variables|Default|GetCardsOnHands) NewItem))

(fn SpendCard
  (params (ItemToFind :type E_SafeItems%20Enum%20%28by%20ref%29 :default "NewEnumerator0"))
  (bind _cardsonhands (Variables|Default|GetCardsOnHands))
  (bind _returnvalue (Utilities|Array|FindItem _cardsonhands ItemToFind))
  (if (>= _returnvalue 0)
    (Utilities|Array|RemoveIndex (Variables|Default|GetCardsOnHands))
    (return _returnvalue)
    (else
      (return _returnvalue))))

(fn GetCardsonHand
  (return (Variables|Default|GetCardsOnHands)))