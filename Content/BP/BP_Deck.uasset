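; BP_Deck is a visual card deck that shows a dummy deck mesh with a separate top card.
; UpdateDeckState looks up mesh scale, mesh position and top card position in maps keyed by graphical state, with one state hiding the deck mesh and lowering the top card.
; MaterialInit creates a dynamic card-face material when none is valid, and UpdateTopCard swaps its CardTop texture.
; The construction script applies a default Ammonit face through a separate material instance.
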(event Custom|UpdateDeckState
  (params (Key :type E_DeckGraphicalState%20Enum%20%28by%20ref%29 :default "NewEnumerator0"))
  (bind _deckscale (Variables|Default|GetDeckScale))
  (bind _deckpos (Variables|Default|GetDeckPos))
  (bind _topcardpos (Variables|Default|GetTopCardPos))
  (bind _value (Utilities|Map|Find _deckscale Key))
  (bind _value_2 (Utilities|Map|Find _topcardpos Key))
  (bind _value_3 (Utilities|Map|Find _deckpos Key))
  (if (Utilities|Enum|Equal(Enum) Key (Utilities|Enum|LiteralenumE_DeckGraphicalState "NewEnumerator3"))
    (Rendering|SetVisibility (Variables|Default|GetDummyDeckMesh) false false)
    (Transformation|SetRelativeLocation (Variables|Default|GetTopCard) (Math|Vector|MakeVector -9.1e-05 -0.095187 -2.0) false false)
    (else
      (Rendering|SetVisibility (Variables|Default|GetDummyDeckMesh) true false)
      (Transformation|SetRelativeScale3D (Variables|Default|GetDummyDeckMesh) (Math|Vector|MakeVector (.x _value) (.y _value) (.z _value)))
      (Transformation|SetRelativeLocation (Variables|Default|GetDummyDeckMesh) (Math|Vector|MakeVector (.x _value_3) (.y _value_3) (.z _value_3)) false false)
      (Transformation|SetRelativeLocation (Variables|Default|GetTopCard) (Math|Vector|MakeVector (.x _value_2) (.y _value_2) (.z _value_2)) false false))))

(event Custom|UpdateTopCard
  (params (Value :type Texture%20Object%20Reference))
  (Rendering|Material|SetTextureParameterValue (Variables|Default|GetMaterialInstance) "CardTop" Value)
  (Rendering|Material|SetMaterial (Variables|Default|GetTopCard) 0 (Variables|Default|GetMaterialInstance)))

(event Custom|MaterialInit
  (Utilities|IsValid (Variables|Default|GetMaterialInstance)
    (:Is%20Not%20Valid
      (bind _returnvalue (Rendering|Material|CreateDynamicMaterialInstance (Variables|Default|GetTopCard) 0 "/Game/Materials/AdvCard_Face.AdvCard_Face" "None" :!class /Script/Engine.PrimitiveComponent))
      (Variables|Default|SetMaterialInstance _returnvalue))))

(fn ConstructionScript
  (bind _returnvalue (Rendering|Material|CreateDynamicMaterialInstance "/Game/Materials/AdvCard_Face.AdvCard_Face" "None" :!class /Script/Engine.KismetMaterialLibrary))
  (Rendering|Material|SetTextureParameterValue _returnvalue "CardTop" "/Game/Textures/Dinos/Faces/Ammonit.Ammonit")
  (Rendering|Material|SetMaterial (Variables|Default|GetTopCard) 0 _returnvalue))