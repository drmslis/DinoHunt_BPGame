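; Player controller for a dinosaur-hunting board game, mapping input actions and debug-style keys to calls on BP_GameMod's objects.
; Inputs roll two dice to move the current player, step one tile, jump a pawn (Fishka), switch deck graphics or print dinos, traps and cards.
; The EndTurn input triggers HuntUI.Hunt, while a separate End Turn function cycles CurrentPlayer.
; The O key bubble-sorts WinnerTable by points and prints the winner.
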(event EventTick
  (params (DeltaSeconds :type Float%20%28single-precision%29)))

(event EventBeginPlay)

(event Input|ActionEvents|InputActionRollDice
  (params (Key :type Key%20Structure :default "None"))
  (:Pressed
    (bind _asbp_game_mod (Utilities|Casting|CastToBP_GameMod (Game|GetGameMode)))
    (bind _output_get (Variables|Default|SetDice1 (Math|Random|RandomIntegerinRange 1 6)))
    (bind _output_get_2 (Variables|Default|SetDice2 (Math|Random|RandomIntegerinRange 1 6)))
    (Development|PrintString (Utilities|String|Append (Utilities|String|ToString(Integer) _output_get) "+" (Utilities|String|ToString(Integer) _output_get_2)) true true "(R=1.000000,G=0.267484,B=0.000000,A=1.000000)" 5.0)
    (Default|MovePlayer (Variables|/Game/BP/BP_GameMod.BP_GameMod_C|GetCurrentPlayerRef _asbp_game_mod) _output_get _output_get_2 false)))

(event Input|ActionEvents|InputActionEndTurn
  (params (Key :type Key%20Structure :default "None"))
  (:Pressed
    (bind _asbp_game_mod (Utilities|Casting|CastToBP_GameMod (Game|GetGameMode)))
    (Default|Hunt (Variables|/Game/BP/BP_GameMod.BP_GameMod_C|GetHuntUI _asbp_game_mod))))

(event Input|ActionEvents|InputActionDrawAdventure
  (params (Key :type Key%20Structure :default "None"))
  (:Pressed
    (bind _asbp_game_mod (Utilities|Casting|CastToBP_GameMod (Game|GetGameMode)))
    (Default|FishkaJump (Utilities|Array|Get(acopy) (Variables|/Game/BP/BP_GameMod.BP_GameMod_C|GetFishkaArray _asbp_game_mod) (Variables|Default|GetCurrentPlayer)) (Utilities|Array|Get(acopy) (Variables|/Game/BP/BP_GameMod.BP_GameMod_C|GetTileArray _asbp_game_mod) 1))))

(event Input|ActionEvents|InputActionDinos
  (params (Key :type Key%20Structure :default "None"))
  (:Pressed
    (bind _asbp_game_mod (Utilities|Casting|CastToBP_GameMod (Game|GetGameMode)))
    (for (_array_element _array_index) (Variables|/Game/BP/Fishka.Fishka_C|GetPlayerDinos (Variables|/Game/BP/BP_GameMod.BP_GameMod_C|GetCurrentPlayerRef _asbp_game_mod))
      (Development|PrintString (Utilities|String|Append (Utilities|String|ToString(Integer) _array_index) ". " (Utilities|String|ToString(Name) (.dinoname _array_element)) " " (Utilities|String|ToString(Integer) (.dinocost _array_element)))))
    (Development|PrintString "Dino List")))

(event Input|ActionEvents|InputActionTraps
  (params (Key :type Key%20Structure :default "None"))
  (:Pressed
    (bind _asbp_game_mod (Utilities|Casting|CastToBP_GameMod (Game|GetGameMode)))
    (for (_array_element _array_index) (Variables|/Game/BP/Fishka.Fishka_C|GetActiveTraps (Variables|/Game/BP/BP_GameMod.BP_GameMod_C|GetCurrentPlayerRef _asbp_game_mod))
      (Development|PrintString (Utilities|String|Append (Utilities|String|ToString(Integer) _array_index) ". " (Utilities|GetDisplayName _array_element))))
    (Development|PrintString "Traps List")))

(event Input|ActionEvents|InputActioninvebtory
  (params (Key :type Key%20Structure :default "None"))
  (:Pressed
    (bind _asbp_game_mod (Utilities|Casting|CastToBP_GameMod (Game|GetGameMode)))
    (for (_array_element _array_index) (Variables|/Game/BP/Fishka.Fishka_C|GetCardsOnHands (Variables|/Game/BP/BP_GameMod.BP_GameMod_C|GetCurrentPlayerRef _asbp_game_mod))
      (Development|PrintString (Utilities|String|Append (Utilities|String|ToString(Integer) _array_index) ". " (Utilities|String|ToString(Name) _array_element))))
    (Development|PrintString "Cards on hands")))

(event Input|KeyboardEvents|1
  (params (Key :type Key%20Structure :default "None"))
  (:Pressed
    (bind _asbp_game_mod (Utilities|Casting|CastToBP_GameMod (Game|GetGameMode)))
    (Default|UpdateDeckState (Variables|/Game/BP/BP_GameMod.BP_GameMod_C|GetDeckObjRef _asbp_game_mod) (Utilities|Enum|LiteralenumE_DeckGraphicalState "NewEnumerator1"))))

(event Input|KeyboardEvents|2
  (params (Key :type Key%20Structure :default "None"))
  (:Pressed
    (bind _asbp_game_mod (Utilities|Casting|CastToBP_GameMod (Game|GetGameMode)))
    (Default|UpdateDeckState (Variables|/Game/BP/BP_GameMod.BP_GameMod_C|GetDeckObjRef _asbp_game_mod) (Utilities|Enum|LiteralenumE_DeckGraphicalState "NewEnumerator2"))))

(event Input|KeyboardEvents|3
  (params (Key :type Key%20Structure :default "None"))
  (:Pressed
    (bind _asbp_game_mod (Utilities|Casting|CastToBP_GameMod (Game|GetGameMode)))
    (Default|UpdateDeckState (Variables|/Game/BP/BP_GameMod.BP_GameMod_C|GetDeckObjRef _asbp_game_mod) (Utilities|Enum|LiteralenumE_DeckGraphicalState "NewEnumerator3"))))

(event Input|KeyboardEvents|0
  (params (Key :type Key%20Structure :default "None"))
  (:Pressed
    (bind _asbp_game_mod (Utilities|Casting|CastToBP_GameMod (Game|GetGameMode)))
    (Default|UpdateDeckState (Variables|/Game/BP/BP_GameMod.BP_GameMod_C|GetDeckObjRef _asbp_game_mod) (Utilities|Enum|LiteralenumE_DeckGraphicalState "NewEnumerator0"))))

(event Input|KeyboardEvents|C
  (params (Key :type Key%20Structure :default "None")))

(event Input|KeyboardEvents|Add
  (params (Key :type Key%20Structure :default "None"))
  (:Pressed
    (bind _asbp_game_mod (Utilities|Casting|CastToBP_GameMod (Game|GetGameMode)))
    (Default|MovePlayer (Variables|/Game/BP/BP_GameMod.BP_GameMod_C|GetCurrentPlayerRef _asbp_game_mod) 1 0 true)))

(event Input|KeyboardEvents|Subtract
  (params (Key :type Key%20Structure :default "None"))
  (:Pressed
    (bind _asbp_game_mod (Utilities|Casting|CastToBP_GameMod (Game|GetGameMode)))
    (Default|MovePlayer (Variables|/Game/BP/BP_GameMod.BP_GameMod_C|GetCurrentPlayerRef _asbp_game_mod) 1 0 false)))

(event Input|KeyboardEvents|O
  (params (Key :type Key%20Structure :default "None"))
  (bind _winnertable (Variables|Default|GetWinnerTable))
  (bind _winnertable_2 (Variables|Default|GetWinnerTable))
  (bind _winnertable_3 (Variables|Default|GetWinnerTable))
  (bind _returnvalue (Utilities|Array|LastIndex _winnertable_2))
  (:Pressed
    (bind _index (Utilities|FlowControl|ForLoopwithBreak 0 (- _returnvalue 1) :!label _label)
      (:LoopBody
        (Variables|Default|SetConter 0)
        (for _index_2 (range 0 (- (- _returnvalue _index) 1))
          (if (< (.points (Utilities|Array|Get(acopy) _winnertable_3 _index_2)) (.points (Utilities|Array|Get(acopy) _winnertable_3 (+ _index_2 1))))
            (Utilities|Array|Swap (Variables|Default|GetWinnerTable) _index_2 (+ _index_2 1))
            (Variables|Default|SetConter 1)))
        (if (== (Variables|Default|GetConter) 0)
          (goto _label Break)))
      (:Completed
        (for _array_element _winnertable
          (Development|PrintString (Utilities|String|Append (Utilities|String|ToString(Name) (.name _array_element)) ". " (Utilities|String|ToString(Integer) (.points _array_element))) true true "(R=0.000000,G=0.660000,B=1.000000,A=1.000000)" 6e+01))
        (Development|PrintString (Utilities|String|ToString(Name) (.name (Utilities|Array|Get(acopy) _winnertable))) true true "(R=1.000000,G=0.053850,B=0.000000,A=1.000000)" 1e+01)))))

(fn ConstructionScript)

(fn PlayerMove
  (bind _asbp_game_mod (Utilities|Casting|CastToBP_GameMod (Game|GetGameMode)))
  (Default|PlayerStep (Utilities|Array|Get(acopy) (Variables|/Game/BP/BP_GameMod.BP_GameMod_C|GetFishkaArray _asbp_game_mod) (Variables|Default|GetCurrentPlayer))))

(fn EndTurn
  (bind _asbp_game_mod (Utilities|Casting|CastToBP_GameMod (Game|GetGameMode)))
  (if (> (Utilities|Array|LastIndex (Variables|/Game/BP/BP_GameMod.BP_GameMod_C|GetFishkaArray _asbp_game_mod)) (Variables|Default|GetCurrentPlayer))
    (Math|Integer|IncrementInt (Variables|Default|GetCurrentPlayer))
    (else
      (Variables|Default|SetCurrentPlayer 0))))

(fn EnterEvent
  (params (NewParam :type Fishka%20Object%20Reference))
  (return false))