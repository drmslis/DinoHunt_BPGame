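; BP_SHTile is a board tile that represents one of four SH types: River, Swamp, Indians or Monkeys.
; On custom tile initialization it sets its sprite to match its SHType.
; When a pawn triggers its enter event, it passes the type to the game mode's SHActivate and returns false, leaving the effect to the game mode.
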(event EventBeginPlay)

(event Collision|EventActorBeginOverlap
  (params (OtherActor :type Actor%20Object%20Reference))
  (|CallParentFunction OtherActor) ; This node is disabled and will not be called.\nDrag off pins to build functionality.
)

(event EventTick
  (params (DeltaSeconds :type Float%20%28single-precision%29))
  (|CallParentFunction DeltaSeconds) ; This node is disabled and will not be called.\nDrag off pins to build functionality.
)

(event EventCustomTileInit
  (switch Utilities|FlowControl|Switch|SwitchonE_SHType (Variables|Default|GetSHType)
    (:NewEnumerator0
      (Rendering|Components|Sprite|SetSprite (Variables|Default|GetTileSprite) "/Game/Sprites/TileSprites/River_Sprite.River_Sprite"))
    (:NewEnumerator1
      (Rendering|Components|Sprite|SetSprite (Variables|Default|GetTileSprite) "/Game/Sprites/TileSprites/Swamp_Sprite.Swamp_Sprite"))
    (:NewEnumerator2
      (Rendering|Components|Sprite|SetSprite (Variables|Default|GetTileSprite) "/Game/Sprites/TileSprites/Indians_Sprite.Indians_Sprite"))
    (:NewEnumerator3
      (Rendering|Components|Sprite|SetSprite (Variables|Default|GetTileSprite) "/Game/Sprites/TileSprites/MonkeysTile_Sprite.MonkeysTile_Sprite"))))

(fn ConstructionScript)

(fn EnterEvent
  (params (ActivePawnRef :type BP%20Pawn%20Object%20Reference))
  (Default|SHActivate (Variables|Default|GetBP_GameModeRef) (Variables|Default|GetSHType))
  (return false))