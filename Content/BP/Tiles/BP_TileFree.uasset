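; Board tile that players can claim with a trap, charging other players diamonds to hunt there.
; EnterEvent starts a hunt for the trap's owner; other players use up a safe card or get a pay or insufficient-diamonds prompt, and unclaimed tiles show a place-trap or no-traps prompt.
; SetTrap, DestroyTrap and PayRent handle ownership, sprite tint and diamond transfer, with BP_GameMod supplying the hunt, stats refresh and TrapManagerUI.
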(event Custom|SetTrap
  (bind _actingplayer (Variables|Default|GetActingPlayer))
  (Sprite|SetSpriteColor (Variables|Default|GetTrapSprite) (Math|Conversions|ToLinearColor(Vector) (Variables|/Game/BP/Fishka.Fishka_C|GetPlayerColor _actingplayer)))
  (Math|Integer|DecrementInt (Variables|/Game/BP/Fishka.Fishka_C|GetTraps _actingplayer)
    (:%20%20
      (bind _output_get (Variables|Default|SetOwnerPlayer (Variables|Default|GetActingPlayer)))
      (Variables|Default|SetTrapOwnerNum (Variables|/Game/BP/Fishka.Fishka_C|GetPlayerNumber _output_get))
      (Utilities|Array|Add (Variables|/Game/BP/Fishka.Fishka_C|GetActiveTraps (Variables|Default|GetActingPlayer)) self)
      (bind _asbp_game_mod (Utilities|Casting|CastToBP_GameMod (Game|GetGameMode)))
      (Default|UPdateStats _asbp_game_mod))))

(event Custom|DestroyTrap
  (Sprite|SetSpriteColor (Variables|Default|GetTrapSprite) "(R=1.000000,G=1.000000,B=1.000000,A=1.000000)")
  (Variables|Default|SetTrapOwnerNum 0))

(event Custom|PayRent
  (bind _actingplayer (Variables|Default|GetActingPlayer))
  (bind _ownerplayer (Variables|Default|GetOwnerPlayer))
  (Variables|/Game/BP/Fishka.Fishka_C|SetDiamonds _actingplayer (- (Variables|/Game/BP/Fishka.Fishka_C|GetDiamonds _actingplayer) 3))
  (Variables|/Game/BP/Fishka.Fishka_C|SetDiamonds _ownerplayer (+ (Variables|/Game/BP/Fishka.Fishka_C|GetDiamonds _ownerplayer) 3))
  (bind _asbp_game_mod (Utilities|Casting|CastToBP_GameMod (Game|GetGameMode)))
  (Default|UPdateStats _asbp_game_mod)
  (Development|PrintString "ВЫЗОВ ОХОТЫ"))

(event EventBeginPlay)

(event Collision|EventActorBeginOverlap
  (params (OtherActor :type Actor%20Object%20Reference))
  (|CallParentFunction OtherActor) ; This node is disabled and will not be called.\nDrag off pins to build functionality.
)

(event EventTick
  (params (DeltaSeconds :type Float%20%28single-precision%29))
  (|CallParentFunction DeltaSeconds) ; This node is disabled and will not be called.\nDrag off pins to build functionality.
)

(fn ConstructionScript)

(fn EnterEvent
  (params (NewParam :type Fishka%20Object%20Reference))
  (bind _output_get (Variables|Default|SetActingPlayer NewParam))
  (if (Math|Conversions|ToBoolean(Integer) (Variables|Default|GetTrapOwnerNum))
    (if (== (Variables|/Game/BP/Fishka.Fishka_C|GetPlayerNumber (Variables|Default|GetActingPlayer)) (Variables|Default|GetTrapOwnerNum))
      (bind _asbp_game_mod (Utilities|Casting|CastToBP_GameMod (Game|GetGameMode)))
      (Default|Hunt _asbp_game_mod)
      (return false)
      (else
        ;[1 1 1] Проверяем сейф-карту. Если есть - охотимся бесплатно
        (bind _array_element (Utilities|Array|ForEachLoopwithBreak (Variables|Default|GetSafeCardsNames) :!label _label)
          (:LoopBody
            (bind (_iscard _cardindex) (Default|IsCardonHand (Variables|Default|GetActingPlayer) _array_element))
            (if _iscard
              (Default|LoseSafeCard (Variables|Default|GetActingPlayer) _array_element _cardindex)
              (Variables|Default|SetFoundSafeCard _array_element)
              (goto _label Break)))
          (:Completed
            (if _iscard
              (bind _asbp_game_mod_2 (Utilities|Casting|CastToBP_GameMod (Game|GetGameMode)))
              (Default|SwitchTrapWidget (Variables|/Game/BP/BP_GameMod.BP_GameMod_C|GetTrapManagerUI _asbp_game_mod_2) 5)
              (Default|ChangeCardName (Variables|/Game/BP/BP_GameMod.BP_GameMod_C|GetTrapManagerUI _asbp_game_mod_2) (Variables|Default|GetFoundSafeCard))
              (Default|ToggleVisibility (Variables|/Game/BP/BP_GameMod.BP_GameMod_C|GetTrapManagerUI _asbp_game_mod_2))
              (elif (>= (Variables|/Game/BP/Fishka.Fishka_C|GetDiamonds (Variables|Default|GetActingPlayer)) 3)
                ;[1 1 1] Есть бабло - запрашиваем охоту в чужом капкане
                (bind _asbp_game_mod_3 (Utilities|Casting|CastToBP_GameMod (Game|GetGameMode)))
                (Default|SwitchTrapWidget (Variables|/Game/BP/BP_GameMod.BP_GameMod_C|GetTrapManagerUI _asbp_game_mod_3) 2)
                (Default|ToggleVisibility (Variables|/Game/BP/BP_GameMod.BP_GameMod_C|GetTrapManagerUI _asbp_game_mod_3))
                (Default|Setter (Variables|/Game/BP/BP_GameMod.BP_GameMod_C|GetTrapManagerUI _asbp_game_mod_3) self)
                (else
                  ;[1 1 1] Нет бабла
                  (bind _asbp_game_mod_4 (Utilities|Casting|CastToBP_GameMod (Game|GetGameMode)))
                  (Default|SwitchTrapWidget (Variables|/Game/BP/BP_GameMod.BP_GameMod_C|GetTrapManagerUI _asbp_game_mod_4) 3)
                  (Default|ToggleVisibility (Variables|/Game/BP/BP_GameMod.BP_GameMod_C|GetTrapManagerUI _asbp_game_mod_4)))))
            (return false)))))
    (else
      (if (> (Variables|/Game/BP/Fishka.Fishka_C|GetTraps _output_get) 0)
        ;[1 1 1] Капканы есть - запрашиваем ставить или нет
        (bind _asbp_game_mod_5 (Utilities|Casting|CastToBP_GameMod (Game|GetGameMode)))
        (Default|SwitchTrapWidget (Variables|/Game/BP/BP_GameMod.BP_GameMod_C|GetTrapManagerUI _asbp_game_mod_5))
        (Default|ToggleVisibility (Variables|/Game/BP/BP_GameMod.BP_GameMod_C|GetTrapManagerUI _asbp_game_mod_5))
        (Default|Setter (Variables|/Game/BP/BP_GameMod.BP_GameMod_C|GetTrapManagerUI _asbp_game_mod_5) self)
        (else
          ;[1 1 1] Нет капкана
          (bind _asbp_game_mod_6 (Utilities|Casting|CastToBP_GameMod (Game|GetGameMode)))
          (Default|SwitchTrapWidget (Variables|/Game/BP/BP_GameMod.BP_GameMod_C|GetTrapManagerUI _asbp_game_mod_6) 1)
          (Default|ToggleVisibility (Variables|/Game/BP/BP_GameMod.BP_GameMod_C|GetTrapManagerUI _asbp_game_mod_6))))
      (return false))))