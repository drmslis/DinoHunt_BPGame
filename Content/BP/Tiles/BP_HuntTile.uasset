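; BP_HuntTile is a board tile where a player can set a trap and collect diamond rent from opponents who land there.
; EnterEvent checks trap ownership, the visitor's safe cards, diamonds and trap count, then hands each outcome to the game mode.
; SetTrap records the owner, tints the sprite their color and ends the turn.
; PayRent transfers diamonds to the owner, while DestroyTrap clears the owner number and tint.
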(event Custom|SetTrap
  (bind _bp_gamemoderef (Variables|Default|GetBP_GameModeRef))
  (Sprite|SetSpriteColor (Variables|Default|GetTrapSprite) (Math|Conversions|ToLinearColor(Vector) (Default|GetPlayerColor (Variables|Default|GetActingPlayer))))
  (Default|SpendTrap (Variables|Default|GetActingPlayer))
  (Variables|Default|SetTrapOwnerNum (Default|GetPlayerNumber (Variables|Default|GetActingPlayer)))
  (Default|AddOwnedTrap (Variables|Default|GetActingPlayer) self)
  (Variables|Default|SetOwnerPlayer (Variables|Default|GetActingPlayer))
  (Default|UPdateStats _bp_gamemoderef)
  (Default|EndTurn _bp_gamemoderef false))

(event Custom|DestroyTrap
  (Sprite|SetSpriteColor (Variables|Default|GetTrapSprite) "(R=1.000000,G=1.000000,B=1.000000,A=1.000000)")
  (Variables|Default|SetTrapOwnerNum 0))

(event Custom|PayRent
  (bind _diamondspayed (Default|SpendDiamonds (Variables|Default|GetActingPlayer) (Variables|Default|GetRent) true false))
  (Default|AddDiamonds (Variables|Default|GetOwnerPlayer) _diamondspayed)
  (Default|UPdateStats (Variables|Default|GetBP_GameModeRef)))

(event EventBeginPlay)

(event Collision|EventActorBeginOverlap
  (params (OtherActor :type Actor%20Object%20Reference))
  (|CallParentFunction OtherActor) ; This node is disabled and will not be called.\nDrag off pins to build functionality.
)

(event EventTick
  (params (DeltaSeconds :type Float%20%28single-precision%29))
  (|CallParentFunction DeltaSeconds) ; This node is disabled and will not be called.\nDrag off pins to build functionality.
)

(fn ConstructionScript)

(fn EnterEvent
  (params (ActivePawnRef :type BP%20Pawn%20Object%20Reference))
  (bind _output_get (Variables|Default|SetActingPlayer ActivePawnRef))
  (if (Math|Conversions|ToBoolean(Integer) (Variables|Default|GetTrapOwnerNum))
    (if (== (Default|GetPlayerNumber (Variables|Default|GetActingPlayer)) (Variables|Default|GetTrapOwnerNum))
      (Default|HuntTile (Variables|Default|GetBP_GameModeRef) false)
      (return false)
      (else
        ;[1 1 1] SafeCardCheck. If no, check diamonds to pay rent
        (bind _array_element (Utilities|Array|ForEachLoopwithBreak (Variables|Default|GetSafeCardsNames) :!label _label)
          (:LoopBody
            (bind _cardindex (Default|IsCardonHand (Variables|Default|GetActingPlayer) _array_element))
            (if (>= _cardindex 0)
              (LocalVariables|SetSafeCardFound _array_element)
              (goto _label Break)))
          (:Completed
            (if (>= _cardindex 0)
              (Default|SpendFreeHuntCard (Variables|Default|GetBP_GameModeRef) (LocalVariables|GetSafeCardFound))
              (elif (>= (Default|GetDiamonds (Variables|Default|GetActingPlayer)) (Variables|Default|GetRent))
                ;[1 1 1] Enough Diamonds. Will pay rent?
                (Default|WillHuntforRent (Variables|Default|GetBP_GameModeRef) self)
                (else
                  ;[1 1 1] Not Enough Diamonds :(
                  (Default|NotEnoughDiamonds (Variables|Default|GetBP_GameModeRef)))))))))
    (elif (> (Default|GetTrapsAmount _output_get) 0)
      ;[1 1 1] You have traps. Will Set?
      (Default|TrapSetInit (Variables|Default|GetBP_GameModeRef) self)
      (else
        ;[1 1 1] NotEnougthTraps
        (Default|TrapNotEnough (Variables|Default|GetBP_GameModeRef))))))