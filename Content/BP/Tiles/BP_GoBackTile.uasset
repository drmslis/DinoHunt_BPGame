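; BP_GoBackTile is a board tile that sends play back when entered.
; EnterEvent calls GoBack on BP_GameMod, passes the tile's GoBakcTypeTile to the EventSolverUI's GoBackSolver, and returns false.
; At game-start preparation, Anomaly and Volkano variants rotate the tile sprite in opposite directions.
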(event Custom|TileStartGamePrepare
  (switch Utilities|FlowControl|Switch|SwitchonGoBackType (Variables|Default|GetGoBakcTypeTile)
    (:NewEnumerator0
      (Transformation|AddLocalRotation (Variables|Default|GetTileSprite) "90.000000,0.000000,0.000000" false false))
    (:NewEnumerator1
      (Transformation|AddLocalRotation (Variables|Default|GetTileSprite) "-90.000000,0.000000,0.000000" false false))))

(event EventBeginPlay
  (|CallParentFunction) ; This node is disabled and will not be called.\nDrag off pins to build functionality.
)

(event Collision|EventActorBeginOverlap
  (params (OtherActor :type Actor%20Object%20Reference))
  (|CallParentFunction OtherActor) ; This node is disabled and will not be called.\nDrag off pins to build functionality.
)

(event EventTick
  (params (DeltaSeconds :type Float%20%28single-precision%29))
  (|CallParentFunction DeltaSeconds) ; This node is disabled and will not be called.\nDrag off pins to build functionality.
)

(fn ConstructionScript
  (|CallParentFunction))

(fn EnterEvent
  (params (NewParam :type Fishka%20Object%20Reference))
  (bind _asbp_game_mod (Utilities|Casting|CastToBP_GameMod (Game|GetGameMode)))
  (Default|GoBack _asbp_game_mod)
  (Default|GoBackSolver (Variables|/Game/BP/BP_GameMod.BP_GameMod_C|GetEventSolverUI _asbp_game_mod) (Variables|Default|GetGoBakcTypeTile))
  (return false))