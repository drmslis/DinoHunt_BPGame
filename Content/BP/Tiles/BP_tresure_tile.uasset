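; BP_tresure_tile is a treasure tile that awards diamonds through its EnterEvent.
; A switch on TreasureTypeTyle picks the Chest or Mines reward, adds it to the passed-in object and prints a Russian-language message.
; Both branches then pass the treasure type to TreasureSolver on the BP_GameMod's EventSolverUI and return false.
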(event EventBeginPlay
  (|CallParentFunction) ; This node is disabled and will not be called.\nDrag off pins to build functionality.
)

(event Collision|EventActorBeginOverlap
  (params (OtherActor :type Actor%20Object%20Reference))
  (|CallParentFunction OtherActor) ; This node is disabled and will not be called.\nDrag off pins to build functionality.
)

(event EventTick
  (params (DeltaSeconds :type Float%20%28single-precision%29))
  (|CallParentFunction DeltaSeconds) ; This node is disabled and will not be called.\nDrag off pins to build functionality.
)

(fn ConstructionScript
  (|CallParentFunction))

(fn EnterEvent
  (params (NewParam :type Fishka%20Object%20Reference))
  (switch Utilities|FlowControl|Switch|SwitchonTresureTileEnum (Variables|Default|GetTreasureTypeTyle)
    (:NewEnumerator0
      (Default|AddDiamonds NewParam 4)
      (Development|PrintString "Вы нашли клад! Получите  4 алмаза!"))
    (:NewEnumerator1
      (Default|AddDiamonds NewParam 6)
      (Development|PrintString "Вы нашли 6 алмазов!")))
  (bind _asbp_game_mod (Utilities|Casting|CastToBP_GameMod (Game|GetGameMode)))
  (Default|TreasureSolver (Variables|/Game/BP/BP_GameMod.BP_GameMod_C|GetEventSolverUI _asbp_game_mod) (Variables|Default|GetTreasureTypeTyle))
  (return false))