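; Board tile for a trouble event (river, swamp, Indians or monkeys) that can cost the entering player turns.
; TroubleSpawn sets the cube material and a name from LostTileType; EnterEvent uses that name to look up the LostData table.
; The player loses a matching safe card if held; otherwise the payment system opens for an affordable buyback, or lost turns are set.
; Outcomes surface through BP_GameMod and its EventSolverUI.
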(event Custom|TroubleSpawn
  (bind _cube (Variables|Default|GetCube))
  (switch Utilities|FlowControl|Switch|SwitchonLostTileEnum (Variables|Default|GetLostTileType)
    (:NewEnumerator0
      (Rendering|Material|SetMaterial _cube 0 "/Game/Materials/TileMaterials/River.River")
      (Variables|Default|SetName "River"))
    (:NewEnumerator1
      (Rendering|Material|SetMaterial _cube 0 "/Game/Materials/TileMaterials/Swamp.Swamp")
      (Variables|Default|SetName "Swamp"))
    (:NewEnumerator2
      (Rendering|Material|SetMaterial _cube 0 "/Game/Materials/TileMaterials/Indians.Indians")
      (Variables|Default|SetName "Indians"))
    (:NewEnumerator3
      (Rendering|Material|SetMaterial _cube 0 "/Game/Materials/TileMaterials/Monkeys.Monkeys")
      (Variables|Default|SetName "Monkeys"))))

(event EventBeginPlay
  (|CallParentFunction))

(event Collision|EventActorBeginOverlap
  (params (OtherActor :type Actor%20Object%20Reference))
  (|CallParentFunction OtherActor) ; This node is disabled and will not be called.\nDrag off pins to build functionality.
)

(event EventTick
  (params (DeltaSeconds :type Float%20%28single-precision%29))
  (|CallParentFunction DeltaSeconds) ; This node is disabled and will not be called.\nDrag off pins to build functionality.
)

(fn ConstructionScript
  (|CallParentFunction))

(fn EnterEvent
  (params (NewParam :type Fishka%20Object%20Reference))
  (bind _returnvalue (Utilities|GetDataTableRow "/Game/BP/Cards/LostData.LostData" (Variables|Default|GetName))
    (:then
      (bind (_iscard _cardindex) (Default|IsCardonHand NewParam (.safeitem _returnvalue)))
      (if _iscard
        (Default|LoseSafeCard NewParam (.safeitem _returnvalue) _cardindex)
        (bind _asbp_game_mod (Utilities|Casting|CastToBP_GameMod (Game|GetGameMode)))
        (Default|SafeCardUsage (Variables|/Game/BP/BP_GameMod.BP_GameMod_C|GetEventSolverUI _asbp_game_mod) (.number _returnvalue))
        (elif (Math|Conversions|ToBoolean(Integer) (.buyback _returnvalue))
          (bind _canpay (Default|CheckDiamonds NewParam (.buyback _returnvalue)))
          (if _canpay
            (bind _asbp_game_mod_2 (Utilities|Casting|CastToBP_GameMod (Game|GetGameMode)))
            (Default|ShowPaymentSystem _asbp_game_mod_2 (Utilities|Name|Equal(Name) (Variables|Default|GetName) "Indians"))
            (else
              (Default|LoseTurnSetter NewParam (.lostturns _returnvalue) :!label _label)
              (bind _asbp_game_mod_3 (Utilities|Casting|CastToBP_GameMod (Game|GetGameMode)))
              (Default|NoSafeItemorMoney (Variables|/Game/BP/BP_GameMod.BP_GameMod_C|GetEventSolverUI _asbp_game_mod_3) (.number _returnvalue))))
          (else
            (goto _label))))
      (return false))
    (:RowNotFound
      (Development|PrintString "Неприятность не выбрана"))))