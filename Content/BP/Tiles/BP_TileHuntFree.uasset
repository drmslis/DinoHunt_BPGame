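; BP_TileHuntFree is a tile Blueprint that, judging by its name, provides a free hunt when entered.
; Its EnterEvent casts the game mode to BP_GameMod, calls Hunt on that game mode's HuntUI and returns false, leaving its input parameter unused.
; The event graph holds only disabled default events, and the construction script just calls the parent.
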(event EventBeginPlay
  (|CallParentFunction) ; This node is disabled and will not be called.\nDrag off pins to build functionality.
)

(event Collision|EventActorBeginOverlap
  (params (OtherActor :type Actor%20Object%20Reference))
  (|CallParentFunction OtherActor) ; This node is disabled and will not be called.\nDrag off pins to build functionality.
)

(event EventTick
  (params (DeltaSeconds :type Float%20%28single-precision%29))
  (|CallParentFunction DeltaSeconds) ; This node is disabled and will not be called.\nDrag off pins to build functionality.
)

(fn ConstructionScript
  (|CallParentFunction))

(fn EnterEvent
  (params (NewParam :type Fishka%20Object%20Reference))
  (bind _asbp_game_mod (Utilities|Casting|CastToBP_GameMod (Game|GetGameMode)))
  (Default|Hunt (Variables|/Game/BP/BP_GameMod.BP_GameMod_C|GetHuntUI _asbp_game_mod))
  (return false))