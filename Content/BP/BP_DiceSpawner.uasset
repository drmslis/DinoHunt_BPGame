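; Dice spawner actor that throws physical dice for a turn-based game and reports the results to the game mode.
; SpawnDice spawns randomly rotated BP_Dice and starts a timer for RerollCheck, which destroys and respawns any die that has not stopped.
; Once two dice are at rest, their values go to TurnMaker with a doubles flag for forward moves, otherwise to CharacterBackJump.
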(event Custom|SpawnDice
  (params (HowManyDices :type Integer) (IsForward :type Boolean))
  (Variables|Default|SetIsForward IsForward)
  (Variables|Default|SetHowManyDicesToRoll HowManyDices)
  (Utilities|Time|SetTimerbyFunctionName 0 "RerollCheck" (Variables|Default|GetRerollTimer))
  (bind _result (Math|Integer|DecrementInt (Variables|Default|GetHowManyDicesToRoll))
    (:%20%20
      (for _index (range 0 _result)
        (bind _returnvalue (Game|SpawnActorfromClass "/Game/BP/BP_Dice.BP_Dice_C" (Math|Transform|MakeTransform (Transformation|GetActorLocation) (Math|Rotator|MakeRotator 0.0 (Math|Random|RandomFloatinRange -9e+01 45.0) (- -9e+01 (Math|Random|RandomFloatinRange -25.0 25.0))) "0.500000,0.500000,0.500000") "AlwaysSpawn" 0 0))
        (Utilities|Array|Add (Variables|Default|GetDiceArray) _returnvalue)))))

(event Custom|RemoveDices
  (for _array_element (Variables|Default|GetDiceArray)
    (Utilities|IsValid _array_element
      (:Is%20Valid
        (Actor|DestroyActor _array_element))))
  (Utilities|Array|Clear (Variables|Default|GetDiceArray)))

(event Custom|RerollCheck
  (Utilities|Array|Clear (Variables|Default|GetDicesReady))
  (for (_array_element _array_index) (Variables|Default|GetDiceArray)
    (if (Variables|/Game/BP/BP_Dice.BP_Dice_C|GetIsStop _array_element)
      (Utilities|Array|Add (Variables|Default|GetDicesReady) (Variables|/Game/BP/BP_Dice.BP_Dice_C|GetIsStop _array_element))
      (else
        (Utilities|IsValid _array_element
          (:Is%20Valid
            (Actor|DestroyActor _array_element)
            (Utilities|Array|RemoveIndex (Variables|Default|GetDiceArray) _array_index)
            (CallFunction|SpawnDice 1 (Variables|Default|GetIsForward)))))))
  (if (== (Utilities|Array|Length (Variables|Default|GetDicesReady)) 2)
    (Utilities|Array|Clear (Variables|Default|GetDicesReady))
    (bind (_dice1 _dice2) (CallFunction|GetResults))
    (if (Variables|Default|GetIsForward)
      (Default|TurnMaker (Variables|Default|GetGameModeRef) _dice1 _dice2 (== _dice1 _dice2))
      (else
        (Default|CharacterBackJump (Variables|Default|GetGameModeRef) _dice1 _dice2)))
    (else
      (Development|PrintString "Reroll!"))))

(event Custom|GetGameModeRef
  (params (GameModeRef :type BP%20Game%20Mod%20Object%20Reference))
  (Variables|Default|SetGameModeRef GameModeRef))

(event EventBeginPlay)

(event Collision|EventActorBeginOverlap
  (params (OtherActor :type Actor%20Object%20Reference)))

(event EventTick
  (params (DeltaSeconds :type Float%20%28single-precision%29)))

(fn ConstructionScript)

(fn GetDiceArray
  (return (Variables|Default|GetDiceArray)))

(fn GetResults
  (LocalVariables|SetFirstDice (Variables|/Game/BP/BP_Dice.BP_Dice_C|GetDiceValue (Utilities|Array|Get(acopy) (Variables|Default|GetDiceArray))))
  (LocalVariables|SetSecondDice (Variables|/Game/BP/BP_Dice.BP_Dice_C|GetDiceValue (Utilities|Array|Get(acopy) (Variables|Default|GetDiceArray) 1)))
  (return (LocalVariables|GetFirstDice) (LocalVariables|GetSecondDice)))