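; Physics-style dice actor that tumbles and reports the value it lands on.
; BeginPlay picks a random rotation, applied every Tick until the mesh overlaps a BP_SurfaceMap.
; A gated Tick watches for zero velocity, then resolves the result once and closes.
; The result comes from the mesh socket with the lowest world Z, converted to DiceValue through SocketToSideMap, and IsStop is set.
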(event OnComponentBeginOverlap(DiceMesh)
  (params (OverlappedComponent :type Primitive%20Component%20Object%20Reference) (OtherActor :type Actor%20Object%20Reference) (OtherComp :type Primitive%20Component%20Object%20Reference) (OtherBodyIndex :type Integer) (bFromSweep :type Boolean) (SweepResult :type Hit%20Result%20Structure%20%28by%20ref%29))
  (bind _asbp_surface_map (Utilities|Casting|CastToBP_SurfaceMap OtherActor))
  (Variables|Default|SetSurfaceMap _asbp_surface_map)
  (Variables|Default|SetAddRotation false))

(event Custom|SetDiceValues
  (for _array_element (Transformation|GetAllSocketNames (Variables|Default|GetDiceMesh))
    (if (not (< (.Z (Math|Vector|BreakVector (Transformation|GetSocketLocation (Variables|Default|GetDiceMesh) _array_element))) (Variables|Default|GetMinZValue)))
      (Variables|Default|SetMinZValue (.Z (Math|Vector|BreakVector (Transformation|GetSocketLocation (Variables|Default|GetDiceMesh) _array_element))))
      (Variables|Default|SetCurrentTopSideName _array_element)))
  (Variables|Default|SetDiceValue (.Value (Utilities|Map|Find (Variables|Default|GetSocketToSideMap) (Variables|Default|GetCurrentTopSideName))))
  (Variables|Default|SetIsStop true))

(event EventBeginPlay
  (Variables|Default|SetRandomRotation (Math|Rotator|MakeRotator (Math|Random|RandomFloatinRange 0.0 5.0) (Math|Random|RandomFloatinRange 0.0 5.0) (Math|Random|RandomFloatinRange 0.0 5.0)))
  (Utilities|FlowControl|Gate true) ; enters at Open
)

(event Collision|EventActorBeginOverlap
  (params (OtherActor :type Actor%20Object%20Reference)))

(event EventTick
  (params (DeltaSeconds :type Float%20%28single-precision%29))
  (Utilities|FlowControl|Gate true :!label _label
    (:Exit
      (if (Variables|Default|GetAddRotation)
        (Class|Actor|AddActorWorldRotation (Variables|Default|GetRandomRotation)))
      (if (Math|Vector|Equal(Vector) (Transformation|GetVelocity) "0, 0, 0" 0.0001)
        (Utilities|FlowControl|Sequence
          (:then_0
            (Utilities|FlowControl|DoOnce false
              (:Completed
                (CallFunction|SetDiceValues))))
          (:then_1
            (goto _label Close)))))))

(fn ConstructionScript)